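; Player character that handles movement, aim, jump and sprint, and fades the screen to black as it nears a BP_FadeActor.
; Overlapping that actor with TriggerSphere starts a looping timer that maps distance to the black alpha on BP_CorePC's HUD; ending overlap clears it.
; Keyboard and gamepad inputs share helpers gated by a LockInput macro, with movement relative to control yaw and gamepad sprint toggling on press.
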(event OnComponentBeginOverlap(TriggerSphere)
  (params (OverlappedComponent :type Primitive%20Component%20Object%20Reference) (OtherActor :type Actor%20Object%20Reference) (OtherComp :type Primitive%20Component%20Object%20Reference) (OtherBodyIndex :type Integer) (bFromSweep :type Boolean) (SweepResult :type Hit%20Result%20Structure%20%28by%20ref%29))
  (bind _asbp_fade_actor (Utilities|Casting|CastToBP_FadeActor OtherActor))
  (bind _returnvalue (Utilities|Time|SetTimerbyEvent (delegate Custom|GetDistance) 0.01 true))
  (Variables|Default|SetGetDistanceHandle _returnvalue))

(event OnComponentEndOverlap(TriggerSphere)
  (params (OverlappedComponent :type Primitive%20Component%20Object%20Reference) (OtherActor :type Actor%20Object%20Reference) (OtherComp :type Primitive%20Component%20Object%20Reference) (OtherBodyIndex :type Integer))
  (Utilities|Casting|CastToBP_FadeActor OtherActor)
  (Utilities|Time|ClearandInvalidateTimerbyHandle (Variables|Default|GetGetDistanceHandle)))

(event Custom|GetDistance
  (bind _corepc (GetSet|GetCorePC))
  (Default|SetBlackAlpha (Variables|/Game/FadeToBlack/Core/BP_CorePC.BP_CorePC_C|GetWbp_HUD _corepc) (Math|Float|MapRangeClamped (Transformation|GetDistanceTo (stale OnComponentBeginOverlap(TriggerSphere) _asbp_fade_actor)) 1e+02 5e+02 1.0 0.0)))

(event EventBeginPlay
  (Variables|Default|SetDefaultSpeed (Variables|/Script/Engine.CharacterMovementComponent|GetMaxWalkSpeed (Variables|Character|GetCharacterMovement))))

(event Input|ActionEvents|InputActionSprint
  (params (Key :type Key%20Structure))
  (:Pressed
    (Utilities|LockInput
      (:false
        (Variables|/Script/Engine.CharacterMovementComponent|SetMaxWalkSpeed (Variables|Character|GetCharacterMovement) (Variables|Default|GetSprintSpeed)))))
  (:Released
    (Variables|/Script/Engine.CharacterMovementComponent|SetMaxWalkSpeed (Variables|Character|GetCharacterMovement) (Variables|Default|GetDefaultSpeed))))

(event Input|ActionEvents|InputActionGP_Jump
  (params (Key :type Key%20Structure))
  (:Pressed
    (Utilities|LockInput
      (:false
        (Character|Jump))))
  (:Released
    (Character|StopJumping)))

(event Input|ActionEvents|InputActionGP_Sprint
  (params (Key :type Key%20Structure))
  (:Pressed
    (Utilities|FlowControl|FlipFlop
      (:A
        (Utilities|LockInput
          (:false
            (Variables|/Script/Engine.CharacterMovementComponent|SetMaxWalkSpeed (Variables|Character|GetCharacterMovement) (Variables|Default|GetSprintSpeed)))))
      (:B
        (Variables|/Script/Engine.CharacterMovementComponent|SetMaxWalkSpeed (Variables|Character|GetCharacterMovement) (Variables|Default|GetDefaultSpeed))))))

(event Input|ActionEvents|InputActionJump
  (params (Key :type Key%20Structure))
  (:Pressed
    (Utilities|LockInput
      (:false
        (Character|Jump))))
  (:Released
    (Character|StopJumping)))

(event Input|AxisEvents|InputAxisMoveForward
  (params (AxisValue :type Float%20%28single-precision%29))
  (CallFunction|AddMovementForward AxisValue))

(event Input|AxisEvents|InputAxisMoveBackward
  (params (AxisValue :type Float%20%28single-precision%29))
  (CallFunction|AddMovementForward AxisValue))

(event Input|AxisEvents|InputAxisGP_XAim
  (params (AxisValue :type Float%20%28single-precision%29))
  (CallFunction|AddYawAim AxisValue))

(event Input|AxisEvents|InputAxisGP_YAim
  (params (AxisValue :type Float%20%28single-precision%29))
  (CallFunction|AddPitchAim AxisValue))

(event Input|AxisEvents|InputAxisStrafeLeft
  (params (AxisValue :type Float%20%28single-precision%29))
  (CallFunction|AddMovementRight AxisValue))

(event Input|AxisEvents|InputAxisStrafeRight
  (params (AxisValue :type Float%20%28single-precision%29))
  (CallFunction|AddMovementRight AxisValue))

(event Input|AxisEvents|InputAxisXAim
  (params (AxisValue :type Float%20%28single-precision%29))
  (CallFunction|AddYawAim AxisValue))

(event Input|AxisEvents|InputAxisYAim
  (params (AxisValue :type Float%20%28single-precision%29))
  (CallFunction|AddPitchAim AxisValue))

(event Input|AxisEvents|InputAxisGP_MoveForward
  (params (AxisValue :type Float%20%28single-precision%29))
  (CallFunction|AddMovementForward AxisValue))

(event Input|AxisEvents|InputAxisGP_MoveBackward
  (params (AxisValue :type Float%20%28single-precision%29))
  (CallFunction|AddMovementForward AxisValue))

(event Input|AxisEvents|InputAxisGP_StrafeLeft
  (params (AxisValue :type Float%20%28single-precision%29))
  (CallFunction|AddMovementRight AxisValue))

(event Input|AxisEvents|InputAxisGP_StrafeRight
  (params (AxisValue :type Float%20%28single-precision%29))
  (CallFunction|AddMovementRight AxisValue))

(fn ConstructionScript)

(fn AddMovementRight
  (params (ScaleValue :type Float%20%28single-precision%29))
  (Utilities|LockInput
    (:false
      (Pawn|Input|AddMovementInput self (Math|Vector|GetRightVector (Math|Rotator|MakeRotator 0.0 0.0 (.yaw (Pawn|GetControlRotation :!class /Script/Engine.Pawn)))) ScaleValue false))))

(fn AddMovementForward
  (params (ScaleValue :type Float%20%28single-precision%29))
  (Utilities|LockInput
    (:false
      (Pawn|Input|AddMovementInput self (Math|Vector|GetForwardVector (Math|Rotator|MakeRotator 0.0 0.0 (.yaw (Pawn|GetControlRotation :!class /Script/Engine.Pawn)))) ScaleValue false))))

(fn AddYawAim
  (params (Val :type Float%20%28single-precision%29))
  (Utilities|LockInput
    (:false
      (Pawn|Input|AddControllerYawInput Val))))

(fn AddPitchAim
  (params (Val :type Float%20%28single-precision%29))
  (Utilities|LockInput
    (:false
      (Pawn|Input|AddControllerPitchInput Val))))

(fn GetCorePC
  (Variables|Default|GetCorePC
    (:then
      _)
    (:else
      (bind _asbp_core_pc (Utilities|Casting|CastToBP_CorePC (Pawn|GetController)))
      (Variables|Default|SetCorePC _asbp_core_pc)))
  (return (Variables|Default|GetCorePC)))